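; Player pawn for a height-score ball game, with a physics Ball that plays an impact-scaled boing sound on hard hits.
; BeginPlay creates the score and restart widgets; StartGame enables ball physics and shows the restart button.
; Tick raises MaxHigh from MaxHighRun, updates the score text and saves the best height to the MainCharacter slot.
; Camera and plank height-follow logic is present but disconnected, so it never runs.
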(event OnComponentHit(Ball)
  (params (HitComponent :type Primitive%20Component%20Object%20Reference) (OtherActor :type Actor%20Object%20Reference) (OtherComp :type Primitive%20Component%20Object%20Reference) (NormalImpulse :type Vector :default "0, 0, 0") (Hit :type Hit%20Result%20Structure%20%28by%20ref%29))
  (bind _returnvalue (Math|Vector|VectorLength NormalImpulse))
  (Math|Float|CompareFloat _returnvalue 5e+01
    (:>
      (Audio|PlaySoundatLocation "/Game/Blueprint/Sound/Boing.Boing" (.Location (Collision|BreakHitResult Hit)) "0, 0, 0" (Math|Float|NormalizetoRange _returnvalue 5e+01 1e+03) 1.0 0.0 0 0 0 0))))

(event Custom|SaveScore
  (bind _maxhigh (Variables|Default|GetMaxHigh))
  (bind _returnvalue (SaveGame|DoesSaveGameExist "MainCharacter"))
  (if _returnvalue
    (bind _returnvalue_2 (SaveGame|LoadGamefromSlot "MainCharacter" :!label _label))
    (bind _assave_score (Utilities|Casting|CastToSaveScore _returnvalue_2))
    (if (not (> (Variables|/Game/Blueprint/Save/SaveScore.SaveScore_C|GetMaxHight _assave_score) _maxhigh))
      (Variables|/Game/Blueprint/Save/SaveScore.SaveScore_C|SetMaxHight _assave_score _maxhigh)
      (SaveGame|SaveGametoSlot _returnvalue_2 "MainCharacter"))
    (else
      (bind _returnvalue_3 (SaveGame|CreateSaveGameObject "/Game/Blueprint/Save/SaveScore.SaveScore_C"))
      (bind _returnvalue_4 (SaveGame|SaveGametoSlot _returnvalue_3 "MainCharacter"))
      (if _returnvalue_4
        (goto _label)))))

(event Custom|StartGame
  (Physics|SetSimulatePhysics (Variables|Default|GetBall) true)
  (Widget|SetVisibility (Variables|/Game/Blueprint/Widget/Restart.Restart_C|GetButton_96 (Variables|Default|GetRestart)) "Visible"))

(event EventBeginPlay
  (bind _returnvalue (UserInterface|CreateWidget "/Game/Blueprint/Widget/Score.Score_C" (Game|GetPlayerController 0)))
  (bind _output_get (Variables|Default|SetScoreWidget _returnvalue))
  (UserInterface|Viewport|AddtoViewport _output_get 0)
  (bind _returnvalue_2 (UserInterface|CreateWidget "/Game/Blueprint/Widget/Restart.Restart_C" (Game|GetPlayerController 0)))
  (bind _output_get_2 (Variables|Default|SetRestart _returnvalue_2))
  (UserInterface|Viewport|AddtoViewport _output_get_2 0))

(event Collision|EventActorBeginOverlap
  (params (OtherActor :type Actor%20Object%20Reference)))

(event EventTick
  (params (DeltaSeconds :type Float%20%28single-precision%29))
  (bind _maxhighrun (Variables|Default|GetMaxHighRun))
  (if (> _maxhighrun (Variables|Default|GetMaxHigh))
    (bind _output_get (Variables|Default|SetMaxHigh _maxhighrun))
    (Default|SetText (Variables|Default|GetScoreWidget) (Utilities|Text|ToText(String) (/ (Class|KismetMathLibrary|ToInt64(Float) _output_get) 100)))
    (CallFunction|SaveScore))
  (Variables|Default|SetDelta%20Seconds DeltaSeconds))

(fn ConstructionScript)