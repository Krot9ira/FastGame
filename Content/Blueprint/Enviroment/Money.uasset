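; Money pickup actor that adds one coin to the player's persistent total when it is destroyed with its Picked flag set.
; BeginPlay binds the OnDestroyed handler, which loads the MainCharacter SaveScore slot, first creating and saving it if missing.
; It increments Money, updates the coin display on the BallPawn's Restart member, then saves the slot.
; The counting happens entirely on destruction, as overlap and tick are disabled here.
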(event Custom|OnDestroyed_Event_0
  (params (DestroyedActor :type Actor%20Object%20Reference))
  (if (Variables|Default|GetPicked)
    (bind _returnvalue (SaveGame|DoesSaveGameExist "MainCharacter"))
    (if _returnvalue
      (bind _returnvalue_2 (SaveGame|LoadGamefromSlot "MainCharacter" :!label _label))
      (bind _assave_score (Utilities|Casting|CastToSaveScore _returnvalue_2))
      (bind _output_get (Variables|/Game/Blueprint/Save/SaveScore.SaveScore_C|SetMoney _assave_score (+ (Variables|/Game/Blueprint/Save/SaveScore.SaveScore_C|GetMoney _assave_score) 1)))
      (bind _asball_pawn (Utilities|Casting|CastToBallPawn (Game|Player|GetPlayerPawn 0)))
      (Default|SetCoins (Variables|/Game/Blueprint/BallPawn.BallPawn_C|GetRestart _asball_pawn) (Utilities|Text|ToText(Integer) _output_get))
      (SaveGame|SaveGametoSlot _returnvalue_2 "MainCharacter")
      (else
        (bind _returnvalue_3 (SaveGame|CreateSaveGameObject "/Game/Blueprint/Save/SaveScore.SaveScore_C"))
        (bind _returnvalue_4 (SaveGame|SaveGametoSlot _returnvalue_3 "MainCharacter"))
        (if _returnvalue_4
          (goto _label))))))

(event EventBeginPlay
  (|CallParentFunction)
  (Game|AssignOnDestroyed (delegate Custom|OnDestroyed_Event_0)))

(event Collision|EventActorBeginOverlap
  (params (OtherActor :type Actor%20Object%20Reference))
  (|CallParentFunction OtherActor) ; This node is disabled and will not be called.\nDrag off pins to build functionality.
)

(event EventTick
  (params (DeltaSeconds :type Float%20%28single-precision%29))
  (|CallParentFunction DeltaSeconds) ; This node is disabled and will not be called.\nDrag off pins to build functionality.
)

(fn ConstructionScript
  (|CallParentFunction))