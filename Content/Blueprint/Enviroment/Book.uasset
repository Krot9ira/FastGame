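; Book environment actor that randomizes its orientation and impulse direction when play begins.
; After running the parent BeginPlay, it lays the static mesh at a fixed roll with a random pitch in 45-degree steps.
; A coin flip then sets the Impulse variable to an upward vector along either positive or negative X.
; The graph only stores Impulse and never applies it; overlap and tick events are disabled.
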(event EventBeginPlay
  (|CallParentFunction)
  (Transformation|SetRelativeRotation (Variables|Default|GetStaticMesh) (Math|Rotator|MakeRotator 9e+01 (Math|Conversions|ToFloat(Integer) (* (Math|Random|RandomInteger 6) 45)) 0.0) false false)
  (if (Math|Random|RandomBool)
    (Variables|Default|SetImpulse "500.000000, 0,500.000000")
    (else
      (Variables|Default|SetImpulse "-500.000000, 0,500.000000"))))

(event Collision|EventActorBeginOverlap
  (params (OtherActor :type Actor%20Object%20Reference))
  (|CallParentFunction OtherActor) ; This node is disabled and will not be called.\nDrag off pins to build functionality.
)

(event EventTick
  (params (DeltaSeconds :type Float%20%28single-precision%29))
  (|CallParentFunction DeltaSeconds) ; This node is disabled and will not be called.\nDrag off pins to build functionality.
)

(fn ConstructionScript
  (|CallParentFunction))