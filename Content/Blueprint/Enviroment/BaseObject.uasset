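; BaseObject is a one-shot environment object that randomly places its mesh within its Box bounds at BeginPlay and reacts to the BallPawn.
; A hit from the pawn fires once, applying a velocity-change impulse to its Ball.
; An overlap with either of the pawn's two static meshes clears Picked instead.
; Both paths share an ending that spawns an emitter, plays a sound and destroys the actor.
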(event OnComponentHit(StaticMesh)
  (params (HitComponent :type Primitive%20Component%20Object%20Reference) (OtherActor :type Actor%20Object%20Reference) (OtherComp :type Primitive%20Component%20Object%20Reference) (NormalImpulse :type Vector :default "0, 0, 0") (Hit :type Hit%20Result%20Structure%20%28by%20ref%29))
  (bind _staticmesh (Variables|Default|GetStaticMesh))
  (bind _returnvalue (Transformation|GetWorldLocation _staticmesh))
  (bind _asball_pawn (Utilities|Casting|CastToBallPawn OtherActor))
  (Utilities|FlowControl|DoOnce false
    (:Completed
      (Physics|AddImpulse (Variables|/Game/Blueprint/BallPawn.BallPawn_C|GetBall _asball_pawn) (Variables|Default|GetImpulse) "None" true)
      (Effects|SpawnEmitteratLocation (Variables|Default|GetEmitter%20Template) _returnvalue)
      (Audio|PlaySoundatLocation (Variables|Default|GetSound) _returnvalue "0, 0, 0" 1.0 1.0 0.0 0 0 0 0)
      (Actor|DestroyActor))))

(event OnComponentBeginOverlap(StaticMesh)
  (params (OverlappedComponent :type Primitive%20Component%20Object%20Reference) (OtherActor :type Actor%20Object%20Reference) (OtherComp :type Primitive%20Component%20Object%20Reference) (OtherBodyIndex :type Integer) (bFromSweep :type Boolean) (SweepResult :type Hit%20Result%20Structure%20%28by%20ref%29))
  (bind _staticmesh (Variables|Default|GetStaticMesh))
  (bind _returnvalue (Transformation|GetWorldLocation _staticmesh))
  (bind _asball_pawn (Utilities|Casting|CastToBallPawn OtherActor))
  (if (or (== OtherComp (Variables|/Game/Blueprint/BallPawn.BallPawn_C|GetStaticMesh _asball_pawn)) (== OtherComp (Variables|/Game/Blueprint/BallPawn.BallPawn_C|GetStaticMesh1 _asball_pawn)))
    (Variables|Default|SetPicked false)
    (Effects|SpawnEmitteratLocation (Variables|Default|GetEmitter%20Template) _returnvalue)
    (Audio|PlaySoundatLocation (Variables|Default|GetSound) _returnvalue "0, 0, 0" 1.0 1.0 0.0 0 0 0 0)
    (Actor|DestroyActor)))

(event EventBeginPlay
  (bind _box (Variables|Default|GetBox))
  (bind (_origin _boxextent) (Collision|GetComponentBounds _box))
  (Transformation|SetWorldLocation (Variables|Default|GetStaticMesh) (Math|Random|RandomPointinBoundingBox _origin _boxextent) false false))

(event Collision|EventActorBeginOverlap
  (params (OtherActor :type Actor%20Object%20Reference)))

(event EventTick
  (params (DeltaSeconds :type Float%20%28single-precision%29)))

(fn ConstructionScript)